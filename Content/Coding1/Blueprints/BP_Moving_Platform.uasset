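; BP_Moving_Platform is an actor whose platform shuttles back and forth between Start and End components.
; It starts on BeginPlay, with a timeline alpha lerping the Platform component's world location between the two endpoints, without sweep.
; When the timeline finishes, it waits briefly, then checks its direction to either reverse or play forward again, producing a continuous loop.
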(event Custom|Reverse
  (bind (_direction _platform_0) (Timeline|Timeline%20from%20A%20to%20B Reverse)
    (:Update
      (Transformation|SetWorldLocation (Variables|Default|GetPlatform) (Math|Vector|Lerp(Vector) (Transformation|GetWorldLocation (Variables|Default|GetStart)) (Transformation|GetWorldLocation (Variables|Default|GetEnd)) _platform_0) false false))
    (:Finished
      (Utilities|FlowControl|Delay 2.0)
      (switch Utilities|FlowControl|Switch|SwitchonETimelineDirection _direction
        (:Forward
          (CallFunction|Reverse))
        (:Backward
          (CallFunction|StartPlatform))))))

(event Custom|Start%20Platform
  (bind (_direction _platform_0) (Timeline|Timeline%20from%20A%20to%20B Play)
    (:Update
      (Transformation|SetWorldLocation (Variables|Default|GetPlatform) (Math|Vector|Lerp(Vector) (Transformation|GetWorldLocation (Variables|Default|GetStart)) (Transformation|GetWorldLocation (Variables|Default|GetEnd)) _platform_0) false false))
    (:Finished
      (Utilities|FlowControl|Delay 2.0)
      (switch Utilities|FlowControl|Switch|SwitchonETimelineDirection _direction
        (:Forward
          (CallFunction|Reverse))
        (:Backward
          (CallFunction|StartPlatform))))))

(event EventBeginPlay
  (CallFunction|StartPlatform))

(event Collision|EventActorBeginOverlap
  (params (OtherActor :type Actor%20Object%20Reference)))

(event EventTick
  (params (DeltaSeconds :type Float%20%28single-precision%29)))

(fn ConstructionScript)