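; BP_Banana is a pickup item that heals the BP_Brian character holding it when used.
; Pickup stores the owner and disables collision, while Drop restores collision and launches the mesh forward; both enable physics simulation.
; Use adds health, drops the item through the owner's BPCInteract component, then destroys it after a short delay.
; Debug prints still call it a flashlight.
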(event EventBeginPlay)

(event Collision|EventActorBeginOverlap
  (params (OtherActor :type Actor%20Object%20Reference)))

(event EventTick
  (params (DeltaSeconds :type Float%20%28single-precision%29)))

(event EventUse
  (bind _asbp_brian (Utilities|Casting|CastToBP_Brian (Variables|Default|GetOwner_0)))
  (Variables|/Game/Coding1/Blueprints/BP_Brian.BP_Brian_C|SetHealth _asbp_brian (+ (Variables|/Game/Coding1/Blueprints/BP_Brian.BP_Brian_C|GetHealth _asbp_brian) 1e+01))
  (Default|TrytoDrop (Variables|/Game/Coding1/Blueprints/BP_Brian.BP_Brian_C|GetBPC_Interact _asbp_brian))
  (Utilities|FlowControl|Delay 0.5)
  (Actor|DestroyActor))

(event EventDrop
  (bind _banana (Variables|Default|GetBanana))
  (bind _banana_2 (Variables|Default|GetBanana))
  (Development|PrintText "Flashlight is being dropped")
  (Collision|SetCollisionEnabled _banana_2 "QueryAndPhysics")
  (Physics|SetSimulatePhysics _banana_2 true)
  (Physics|AddImpulse _banana (* (Math|Vector|GetForwardVector _banana) 5e+02) "None" true))

(event EventPickup
  (params (Owner :type Actor%20Object%20Reference))
  (bind _banana (Variables|Default|GetBanana))
  (Variables|Default|SetOwner_0 Owner)
  (Development|PrintText "Flashlight is being picked up")
  (Collision|SetCollisionEnabled _banana "NoCollision")
  (Physics|SetSimulatePhysics _banana true))

(fn ConstructionScript)