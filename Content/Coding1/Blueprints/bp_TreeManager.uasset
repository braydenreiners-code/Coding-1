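; Tree manager actor that animates and staged-reveals every BP_Tree in the level.
; On BeginPlay it waits briefly, caches all trees in an array, starts the leaf wiggle, then hides them all.
; WiggleLeaves re-calls itself after a delay, randomly nudging the current scale of each tree's Sphere child components.
; ShowTreeSlowly unhides trees one at a time through a delayed index loop.
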(event Custom|Wiggle%20Leaves
  (for _array_element (Variables|Default|GetTree%20Array)
    (for _array_element_2 (Components|GetChildrenComponents (Variables|/Game/Coding1/Blueprints/BP_Tree.BP_Tree_C|GetSphere _array_element) true)
      (Transformation|SetRelativeScale3D _array_element_2 (* (Variables|/Script/Engine.SceneComponent|GetRelativeScale3D _array_element_2) (Math|Random|RandomFloatinRange 0.98 1.02)))))
  (Utilities|FlowControl|Delay 0.8)
  (CallFunction|WiggleLeaves))

(event Custom|Hide%20Trees
  (for _array_element (Variables|Default|GetTree%20Array)
    (Rendering|SetActorHiddenInGame _array_element true) ; Hide Tree
  ))

(event Custom|Show%20Tree%20Slowly
  (bind _index (Variables|Default|GetIndex))
  (Utilities|FlowControl|Delay 0.25 :!label _label)
  (Rendering|SetActorHiddenInGame (Utilities|Array|Get(acopy) (Variables|Default|GetTree%20Array) _index) false)
  (Math|Integer|IncrementInt _index ; add 1 to index
    (:%20%20
      (if (not (== (Variables|Default|GetIndex) (Utilities|Array|Length (Variables|Default|GetTree%20Array))))
        (goto _label)))))

(event EventBeginPlay
  (Development|PrintText "Tree Manager starting up") ; text should appear when starting up
  (Utilities|FlowControl|Delay 3.0)
  (Development|PrintText "Delay up")
  (bind _outactors (Actor|GetAllActorsOfClass "/Game/Coding1/Blueprints/BP_Tree.BP_Tree_C"))
  (Variables|Default|SetTree%20Array _outactors)
  (CallFunction|WiggleLeaves)
  (CallFunction|HideTrees)
  (CallFunction|ShowTreeSlowly))

(fn ConstructionScript)