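; BP_Spawner is a spawner actor that creates a configurable class at its SpawnPoint component.
; When AutoSpawn is set, BeginPlay waits briefly and calls SpawnThing, which then re-calls itself after a shorter delay to form a repeating loop.
; SpawnThing can also act as a one-shot spawn when AutoSpawn is off, and it skips spawning if the spot is colliding.
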(event Custom|Spawn%20Thing
  (Game|SpawnActorfromClass (Variables|Default|GetThing%20To%20Spawn) (Transformation|GetWorldTransform (Variables|Default|GetSpawn%20Point)) "DontSpawnIfColliding" "MultiplyWithRoot" 0 0)
  (if (Variables|Default|GetAuto-Spawn)
    (Utilities|FlowControl|Delay 5.0)
    (CallFunction|SpawnThing)))

(event EventBeginPlay
  (Development|PrintText "Spawner Active")
  (if (Variables|Default|GetAuto-Spawn)
    (Utilities|FlowControl|Delay 1e+01)
    (CallFunction|SpawnThing)))

(fn ConstructionScript)