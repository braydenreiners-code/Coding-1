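; BP_DeathPlain is a death pit trigger that ends the run when the player character BP_Brian overlaps its DeathPlain component.
; On overlap it disables Brian's input and reveals the game over and death pit labels on the HUD widget reached through NewHUD.
; After a ten-second delay it restarts the game by reopening the current level by name.
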(event OnComponentBeginOverlap(DeathPlain)
  (params (OverlappedComponent :type Primitive%20Component%20Object%20Reference) (OtherActor :type Actor%20Object%20Reference) (OtherComp :type Primitive%20Component%20Object%20Reference) (OtherBodyIndex :type Integer) (bFromSweep :type Boolean) (SweepResult :type Hit%20Result%20Structure%20%28by%20ref%29))
  (bind _asbp_brian (Utilities|Casting|CastToBP_Brian OtherActor))
  (Input|DisableInput _asbp_brian (Game|GetPlayerController 0))
  (bind _asnew_hud (Utilities|Casting|CastToNewHUD (HUD|GetHUD (Game|GetPlayerController 0))))
  (Variables|/Script/UMG.Widget|SetVisibility (Variables|/Game/Coding1/Widget/W_UI.W_UI_C|GetLabal_GameOver (Variables|/Game/Coding1/Widget/NewHUD.NewHUD_C|GetHUD_Ref _asnew_hud)) "Visible")
  (Variables|/Script/UMG.Widget|SetVisibility (Variables|/Game/Coding1/Widget/W_UI.W_UI_C|GetLabel_Deathpit (Variables|/Game/Coding1/Widget/NewHUD.NewHUD_C|GetHUD_Ref _asnew_hud)) "Visible")
  (Utilities|FlowControl|Delay 1e+01)
  (bind _returnvalue (Game|GetCurrentLevelName true))
  (Game|OpenLevel(byName) (Utilities|String|StringToName _returnvalue)))

(event EventBeginPlay)

(event Collision|EventActorBeginOverlap
  (params (OtherActor :type Actor%20Object%20Reference)))

(event EventTick
  (params (DeltaSeconds :type Float%20%28single-precision%29)))

(fn ConstructionScript)