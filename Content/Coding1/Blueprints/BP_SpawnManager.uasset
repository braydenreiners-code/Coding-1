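; Spawn manager that triggers the level's BP_Spawner actors one at a time, five seconds apart.
; On BeginPlay it gathers every spawner, then a self-calling event steps through the array, calling SpawnThing on each.
; Spawners flagged AutoSpawn are skipped immediately without a delay.
; The array is shuffled and the index reset after each full pass, so only the first pass follows the gathered order.
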(event Custom|Spawn%20a%20thing
  (if (>= (Variables|Default|GetIndex) (Utilities|Array|Length (Variables|Default|GetSpawners))) ; are we at the end of our array?
    (Utilities|Array|Shuffle (Variables|Default|GetSpawners))
    (Variables|Default|SetIndex 0))
  (if (Variables|/Game/Coding1/Blueprints/BP_Spawner.BP_Spawner_C|GetAuto-Spawn (Utilities|Array|Get(acopy) (Variables|Default|GetSpawners) (Variables|Default|GetIndex)))
    (Math|Integer|IncrementInt (Variables|Default|GetIndex)
      (:%20%20
        (CallFunction|SpawnAThing)))
    (else
      (Default|SpawnThing (Utilities|Array|Get(acopy) (Variables|Default|GetSpawners) (Variables|Default|GetIndex)))
      (Math|Integer|IncrementInt (Variables|Default|GetIndex)
        (:%20%20
          (Utilities|FlowControl|Delay 5.0)
          (CallFunction|SpawnAThing))))))

(event EventBeginPlay
  (bind _outactors (Actor|GetAllActorsOfClass "/Game/Coding1/Blueprints/BP_Spawner.BP_Spawner_C")) ; get all the spawners
  (Variables|Default|SetSpawners _outactors)
  (CallFunction|SpawnAThing))

(fn ConstructionScript)